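; BP_Particle is an actor that drives a Niagara particle system whose spawn count comes from an external config file.
; On BeginPlay it reads particles.txt, stores the value as ParticleNumber and passes it as an integer to the User.Spawn Count parameter.
; It then creates a BP_InfoDisplay widget for the first player, showing that number on screen.
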(event `self.ReceiveBeginPlay`
  (bind _returnvalue (`MyBlueprintFunctionLibrary.ReadConfigFile` "particles.txt"))
  (bind _output_get (set `self.particle number` _returnvalue))
  (`NiagaraComponent.SetNiagaraVariableInt` (`self.Niagara`) "User.Spawn Count" (`KismetStringLibrary.Conv_StringToInt` _output_get))
  (bind _returnvalue_2 (`|CreateWidget` "/Game/Blueprints/BP_InfoDisplay.BP_InfoDisplay_C" (`GameplayStatics.GetPlayerController` 0)))
  (set `/Game/Blueprints/BP_InfoDisplay.InfoText` (`KismetTextLibrary.Conv_StringToText` (`self.particle number`)) _returnvalue_2)
  (`UserWidget.AddToViewport` _returnvalue_2 0))

(event `self.ReceiveTick`
  (params (DeltaSeconds :type "Float (single-precision)")))

(fn `UserConstructionScript`)