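; Test actor that fires a configurable number of line traces every frame, apparently as a raycast load test.
; BeginPlay reads the ray count from rays.txt and shows it in a BP_InfoDisplay widget.
; Tick casts Visibility traces from the actor in an evenly spaced horizontal ring of radius R, without using the hit results.
; Trace debug drawing is off, and a DrawDebugLine node is left unconnected.
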(event `self.ReceiveBeginPlay`
  (bind _returnvalue (`MyBlueprintFunctionLibrary.ReadConfigFile` "rays.txt"))
  (set `self.lineNum` (`KismetStringLibrary.Conv_StringToInt` _returnvalue))
  (bind _returnvalue_2 (`|CreateWidget` "/Game/Blueprints/BP_InfoDisplay.BP_InfoDisplay_C" (`GameplayStatics.GetPlayerController` 0)))
  (bind _output_get (set `self.UIWidget` _returnvalue_2))
  (`UserWidget.AddToViewport` _output_get 0)
  (set `/Game/Blueprints/BP_InfoDisplay.InfoText` (`KismetTextLibrary.Conv_IntToText` (`self.lineNum`)) _output_get))

(event `self.ReceiveTick`
  (params (DeltaSeconds :type "Float (single-precision)"))
  (bind _returnvalue (`self.K2_GetActorLocation`))
  (for _index (range (+ (`self.lineNum`) 1))
    (bind _returnvalue_2 (* _index (/ 360.0 (`KismetMathLibrary.Conv_IntToDouble` (`self.lineNum`)))))
    (`KismetSystemLibrary.LineTraceSingle` _returnvalue (`KismetMathLibrary.MakeVector` (+ (.x _returnvalue) (* (`self.r`) (`KismetMathLibrary.DegSin` _returnvalue_2))) (+ (.y _returnvalue) (* (`self.r`) (`KismetMathLibrary.DegCos` _returnvalue_2))) (.z _returnvalue)) "TraceTypeQuery1")))

(fn `UserConstructionScript`)